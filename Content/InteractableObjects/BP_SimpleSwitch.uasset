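; BP_SimpleSwitch is an interactable switch actor that toggles between On and Off.
; Interact flips its Status and plays or reverses the SimpleSwitchMechanics timeline, which rolls the static mesh to animate the switch.
; ShowInfo sets HUD prompt text telling the player to press x to switch it on or off, based on the current Status.
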(event `/Game/AdditionalLogic/I_Interactable.Interact`
  (switch `/Game/InteractableObjects/E_SimpleSwitchStatus` (`self.Status`)
    (:`NewEnumerator0`
      (set `self.Status` "NewEnumerator1")
      (bind (_direction _simpleswitchrotation) (`Timeline|SimpleSwitchMechanics` :!label _label)
        (:`Update`
          (`SceneComponent.K2_SetRelativeRotation` (`self.StaticMesh`) (`KismetMathLibrary.MakeRotator` _simpleswitchrotation) false false))))
    (:`NewEnumerator1`
      (set `self.Status` "NewEnumerator0")
      (goto _label :!via `Reverse`))))

(event `/Game/AdditionalLogic/I_Interactable.ShowInfo`
  (params (HUD :type "/Game/Widgets/WBP_HUD Object Reference"))
  (switch `/Game/InteractableObjects/E_SimpleSwitchStatus` (`self.Status`)
    (:`NewEnumerator0`
      (`/Game/Widgets/WBP_HUD.SetInfoText` HUD "Press x to switch on"))
    (:`NewEnumerator1`
      (`/Game/Widgets/WBP_HUD.SetInfoText` HUD "Press x to switch off"))))

(fn `UserConstructionScript`)