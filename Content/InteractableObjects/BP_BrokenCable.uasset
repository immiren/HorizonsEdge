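; BP_BrokenCable is an interactable broken cable that the player can fix.
; While it is Broken, ShowInfo puts a fix prompt on the HUD and Interact switches it to Fixed.
; Fixing plays the CableMechanics timeline, which drives the static mesh's relative yaw and plays a 2D zap sound when it finishes.
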(event `/Game/InteractableObjects/AdditionalLogic/I_Interactable.Interact`
  (switch `/Game/InteractableObjects/En_BrokenCableStatus` (`self.Status`)
    (:`NewEnumerator0`
      (set `self.Status` "NewEnumerator1")
      (bind (_direction _cable_movement) (`Timeline|CableMechanics`)
        (:`Update`
          (`SceneComponent.K2_SetRelativeLocationAndRotation` (`self.StaticMesh`) (0.0 0.0 0.0) (`KismetMathLibrary.MakeRotator` 0.0 0.0 _cable_movement) false false))
        (:`Finished`
          (`GameplayStatics.SpawnSound2D` "/Game/InteractableObjects/Zap_Cue.Zap_Cue" 1.0 1.0 0.0 null))))))

(event `/Game/InteractableObjects/AdditionalLogic/I_Interactable.ShowInfo`
  (params (HUD :type "/Game/Widgets/WBP_HUD Object Reference"))
  (switch `/Game/InteractableObjects/En_BrokenCableStatus` (`self.Status`)
    (:`NewEnumerator0`
      (`/Game/Widgets/WBP_HUD.SetInfoText` HUD "Press x to fix"))))

(fn `UserConstructionScript`)